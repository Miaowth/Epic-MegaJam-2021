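; Manager actor that lets paused collapsing walls wear down and destroy the actors blocking them.
; On BeginPlay it caches every CollapsingWall_BP and starts a one-second looping TickHealth timer.
; Each pass subtracts a wall's DamagePower from its blockers' Health and destroys those below zero.
; A second pass prunes invalid references from shared blockers, and any wall left without blockers is unblocked.
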(event Custom|Tick%20Health
  (CallFunction|TickHealth))

(event EventBeginPlay
  (bind _outactors (Actor|GetAllActorsOfClass "/Game/MyBlueprints/CollapsingWall_BP.CollapsingWall_BP_C"))
  (Variables|Default|SetCollapsingWallArray _outactors)
  (Utilities|Time|SetTimerbyEvent (delegate Custom|Tick%20Health) 1.0 true))

(event Collision|EventActorBeginOverlap
  (params (OtherActor :type Actor%20Object%20Reference)))

(event EventTick
  (params (DeltaSeconds :type Float%20%28single-precision%29)))

(fn ConstructionScript)

(fn TickHealth
  (bind _aliveblocks (LocalVariables|GetAliveBlocks))
  (bind _aliveblocks_2 (LocalVariables|GetAliveBlocks))
  (for _array_element (Variables|Default|GetCollapsingWallArray)
    (if (Variables|/Game/MyBlueprints/CollapsingWall_BP.CollapsingWall_BP_C|GetIsPaused _array_element)
      (for _array_element_2 (Variables|/Game/MyBlueprints/CollapsingWall_BP.CollapsingWall_BP_C|GetBlocking%20Actors _array_element)
        (bind _output_get (Variables|/Script/UnrealMegaJam.BasePickupObject|SetHealth _array_element_2 (- (Variables|/Script/UnrealMegaJam.BasePickupObject|GetHealth _array_element_2) (Variables|/Script/UnrealMegaJam.CollapsingWall|GetDamagePower _array_element))))
        (Development|PrintString (Utilities|String|ToString(Integer) _output_get))
        (if (>= _output_get 0)
          (Utilities|Array|Add (LocalVariables|GetAliveBlocks) _array_element_2)
          (else
            (Utilities|Array|AddUnique (LocalVariables|GetDestroyBlocks) _array_element_2))))
      (bind _output_get_2 (Variables|/Game/MyBlueprints/CollapsingWall_BP.CollapsingWall_BP_C|SetBlocking%20Actors _array_element _aliveblocks))
      (Utilities|Array|Clear _aliveblocks)
      (if (== (Utilities|Array|Length _output_get_2) 0)
        (Development|PrintString "No Longer Blocked")
        (Default|UnBlockWall _array_element))))
  (for _array_element_3 (LocalVariables|GetDestroyBlocks)
    (Actor|DestroyActor _array_element_3))
  (for _array_element_4 (Variables|Default|GetCollapsingWallArray)
    (if (Variables|/Game/MyBlueprints/CollapsingWall_BP.CollapsingWall_BP_C|GetIsPaused _array_element_4)
      (for _array_element_5 (Variables|/Game/MyBlueprints/CollapsingWall_BP.CollapsingWall_BP_C|GetBlocking%20Actors _array_element_4)
        (if (Utilities|IsValid _array_element_5)
          (Utilities|Array|Add (LocalVariables|GetAliveBlocks) _array_element_5)
          (else
            (Development|PrintString "uwuw fucky wucky ducky"))))
      (bind _output_get_3 (Variables|/Game/MyBlueprints/CollapsingWall_BP.CollapsingWall_BP_C|SetBlocking%20Actors _array_element_4 _aliveblocks_2))
      (Utilities|Array|Clear _aliveblocks_2)
      (if (== (Utilities|Array|Length _output_get_3) 0)
        (Development|PrintString "No Longer Blocked")
        (Default|UnBlockWall _array_element_4)))))