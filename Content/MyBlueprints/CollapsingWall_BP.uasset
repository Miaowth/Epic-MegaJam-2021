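; CollapsingWall actor that moves its wall model from its placed pose to a destination marker as soon as play begins.
; BeginPlay caches the start transform and builds a target from the marker's location and rotation, keeping the wall's original scale.
; A timeline track drives the transform lerp without sweeping, with play rate divided by Speed, so higher values mean slower motion.
; A debug string prints when the timeline finishes.
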(event EventBeginPlay
  (bind _destinationmarker (Variables|Default|GetDestinationMarker))
  (bind _timeline_0 (Variables|Default|GetTimeline_0))
  (bind _returnvalue (Transformation|GetWorldTransform _destinationmarker))
  (bind _output_get (Variables|Default|SetStartingPoint (Transformation|GetWorldTransform (Variables|Default|GetWallModel))))
  (Variables|Default|SetTargetPoint (Math|Transform|MakeTransform (.location _returnvalue) (.rotation _returnvalue) (.scale _output_get)))
  (Components|Timeline|SetPlayRate _timeline_0 (/ (Components|Animation|GetPlayRate _timeline_0) (Variables|Default|GetSpeed)))
  (bind _newtrack_0 (Timeline|Timeline_0 PlayFromStart)
    (:Update
      (Transformation|SetWorldTransform (Variables|Default|GetWallModel) (Math|Transform|Lerp(Transform) (Variables|Default|GetStartingPoint) (Variables|Default|GetTargetPoint) _newtrack_0) false false))
    (:Finished
      (Development|PrintString "Ded"))))

(event Collision|EventActorBeginOverlap
  (params (OtherActor :type Actor%20Object%20Reference)))

(event EventTick
  (params (DeltaSeconds :type Float%20%28single-precision%29)))

(fn ConstructionScript)