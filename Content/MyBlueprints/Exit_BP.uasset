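; Exit actor that decides whether a level is won or lost, in a game with collapsing walls.
; A ThirdPersonCharacter overlapping ActualExit shows the LevelWin widget and reverses the timelines of all CollapsingWall_BP actors cached on BeginPlay.
; A collapsing wall ending its overlap with the actor shows LevelLose instead.
; Both outcomes pass the level name to the widget, switch to UI-only input with cursor and pause the game.
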(event OnComponentBeginOverlap(ActualExit)
  (params (OverlappedComponent :type Primitive%20Component%20Object%20Reference) (OtherActor :type Actor%20Object%20Reference) (OtherComp :type Primitive%20Component%20Object%20Reference) (OtherBodyIndex :type Integer) (bFromSweep :type Boolean) (SweepResult :type Hit%20Result%20Structure%20%28by%20ref%29))
  (bind _returnvalue (Game|GetPlayerController 0))
  (Utilities|Casting|CastToThirdPersonCharacter OtherActor)
  (Development|PrintString "Win uwu")
  (bind _returnvalue_2 (UserInterface|CreateWidget "/Game/UI/LevelWin.LevelWin_C"))
  (bind _returnvalue_3 (Game|GetCurrentLevelName true))
  (Variables|/Game/UI/LevelWin.LevelWin_C|SetCurrentLevelName _returnvalue_2 _returnvalue_3)
  (UserInterface|Viewport|AddtoViewport _returnvalue_2 0)
  (Input|SetInputModeUIOnly _returnvalue _returnvalue_2 "DoNotLock")
  (Variables|/Script/Engine.PlayerController|SetbShowMouseCursor _returnvalue true)
  (for _array_element (Variables|Default|GetWallArray)
    (Utilities|String|Reverse (Variables|/Game/MyBlueprints/CollapsingWall_BP.CollapsingWall_BP_C|GetTimeline_0 _array_element)))
  (Game|SetGamePaused true))

(event EventBeginPlay
  (bind _outactors (Actor|GetAllActorsOfClass "/Game/MyBlueprints/CollapsingWall_BP.CollapsingWall_BP_C"))
  (Variables|Default|SetWallArray _outactors))

(event Collision|EventActorEndOverlap
  (params (OtherActor :type Actor%20Object%20Reference))
  (bind _returnvalue (Game|GetPlayerController 0))
  (Utilities|Casting|CastToCollapsingWall_BP OtherActor)
  (Development|PrintString "ded owo")
  (bind _returnvalue_2 (UserInterface|CreateWidget "/Game/UI/LevelLose.LevelLose_C"))
  (bind _returnvalue_3 (Game|GetCurrentLevelName true))
  (Variables|/Game/UI/LevelLose.LevelLose_C|SetCurrentLevelName _returnvalue_2 _returnvalue_3)
  (UserInterface|Viewport|AddtoViewport _returnvalue_2 0)
  (Input|SetInputModeUIOnly _returnvalue _returnvalue_2 "DoNotLock")
  (Variables|/Script/Engine.PlayerController|SetbShowMouseCursor _returnvalue true)
  (Game|SetGamePaused true))

(event EventTick
  (params (DeltaSeconds :type Float%20%28single-precision%29)))

(fn ConstructionScript)